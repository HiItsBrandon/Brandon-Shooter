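; Actor component that makes its owner's root primitive hover above surfaces and keep itself upright using physics.
; Each tick, a downward Visibility trace applies upward force that fades linearly from max thrust to zero over the trace length.
; An angular impulse also rotates the body's up vector toward world up, using their cross product as axis and scaling strength down as alignment improves.
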(event EventBeginPlay
  ;[1 1 1] BeginPlay
  (bind _asprimitive_component (Utilities|Casting|CastToPrimitiveComponent (Variables|/Script/Engine.Actor|GetRootComponent (Components|GetOwner))))
  (Variables|Default|SetPrimitiveComponent _asprimitive_component))

(event EventTick
  (params (DeltaSeconds :type Float%20%28single-precision%29))
  ;[1 1 1] Tick
  (CallFunction|Hover)
  (CallFunction|Orient))

(fn Hover
  (bind _primitivecomponent (Variables|Default|GetPrimitiveComponent))
  (bind _returnvalue (Transformation|GetWorldLocation _primitivecomponent))
  (bind (_outhit _returnvalue_2) (Collision|LineTraceByChannel _returnvalue (- _returnvalue (Math|Vector|MakeVector 0.0 0.0 (Variables|Default|GetTraceLength))) "TraceTypeQuery1" false 0 "None"))
  (if _returnvalue_2
    (Physics|AddForce (Variables|Default|GetPrimitiveComponent) (* "0, 0,1.000000" (Math|Float|Lerp (Variables|Default|GetMaxThrustStrength) 0.0 (/ (Math|Vector|VectorLength (- (.Location (Collision|BreakHitResult _outhit)) (Transformation|GetWorldLocation (Variables|Default|GetPrimitiveComponent)))) (Variables|Default|GetTraceLength)))) "None" false)))

(fn Orient
  (bind _primitivecomponent (Variables|Default|GetPrimitiveComponent))
  (bind _returnvalue (Transformation|GetWorldRotation _primitivecomponent))
  (bind _returnvalue_2 (Math|Vector|GetUpVector _returnvalue))
  (bind _returnvalue_3 (* _returnvalue_2 -1.0))
  (Class|PrimitiveComponent|AddAngularImpulseinRadians (Variables|Default|GetPrimitiveComponent) (* (Math|Vector|CrossProduct _returnvalue_3 "0, 0,-1.000000") (Math|Float|Lerp (Variables|Default|GetMaxRotationStrength) 0.0 (/ (+ (Math|Vector|DotProduct _returnvalue_3 "0, 0,-1.000000") 1.0) 2.0))) "None" false))