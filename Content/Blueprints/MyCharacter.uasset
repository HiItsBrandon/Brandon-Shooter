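; MyCharacter is a player character Blueprint that handles basic movement and camera look through input axis events.
; The vertical and horizontal move axes add movement input along the forward and right vectors of the full control rotation, pitch included.
; The mouse axes feed controller pitch and yaw, so looking around also steers movement direction.
; The construction script is empty.
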(event Input|AxisEvents|InputAxisMouse_Vertical
  (params (AxisValue :type Float%20%28single-precision%29))
  ;[1 1 1] CharacterLook
  (Pawn|Input|AddControllerPitchInput AxisValue))

(event Input|AxisEvents|InputAxisMouse_Horizontal
  (params (AxisValue :type Float%20%28single-precision%29))
  ;[1 1 1] CharacterLook
  (Pawn|Input|AddControllerYawInput AxisValue))

(event Input|AxisEvents|InputAxisMove_Vertical
  (params (AxisValue :type Float%20%28single-precision%29))
  ;[1 1 1] CharacterMovement
  (Pawn|Input|AddMovementInput (Math|Vector|GetForwardVector (Pawn|GetControlRotation :!class /Script/Engine.Pawn)) AxisValue false))

(event Input|AxisEvents|InputAxisMove_Horizontal
  (params (AxisValue :type Float%20%28single-precision%29))
  ;[1 1 1] CharacterMovement
  (Pawn|Input|AddMovementInput (Math|Vector|GetRightVector (Pawn|GetControlRotation :!class /Script/Engine.Pawn)) AxisValue false))

(fn ConstructionScript)